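; BP_Maze is a tiltable maze puzzle that the player rotates through Enhanced Input.
; On BeginPlay it adds the IMC_Puzzleame mapping context to the BP_PlayerController's input subsystem.
; IA_Rotate applies world rotation to the Cube in roll and inverted pitch, with no clamping.
; A Box overlap by the player pawn serves as the win trigger, currently only printing a "gane" message.
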(event OnComponentBeginOverlap(Box)
  (params (OverlappedComponent :type Primitive%20Component%20Object%20Reference) (OtherActor :type Actor%20Object%20Reference) (OtherComp :type Primitive%20Component%20Object%20Reference) (OtherBodyIndex :type Integer) (bFromSweep :type Boolean) (SweepResult :type Hit%20Result%20Structure%20%28by%20ref%29))
  (if (== OtherActor (Game|Player|GetPlayerPawn 0))
    (Development|PrintString "gane")))

(event Input|EnhancedActionEvents|EnhancedInputActionIA_Rotate
  (params (ActionValue :type Vector%202D%20Structure) (ElapsedSeconds :type Float%20%28double-precision%29) (TriggeredSeconds :type Float%20%28double-precision%29) (InputAction :type Input%20Action%20Object%20Reference :default "/Game/Input/IA_Rotate.IA_Rotate"))
  (:Triggered
    (Transformation|AddWorldRotation (Variables|Default|GetCube) (Math|Rotator|MakeRotator (.x ActionValue) (* (.y ActionValue) -1.0) 0.0) false false)))

(event EventBeginPlay
  (bind _asbp_player_controller (Utilities|Casting|CastToBP_PlayerController (Game|GetPlayerController 0)))
  (Input|AddMappingContext (PlayerController|LocalPlayerSubsystems|GetEnhancedInputLocalPlayerSubsystem _asbp_player_controller) "/Game/Input/IMC_Puzzleame.IMC_Puzzleame" 0 "(bIgnoreAllPressedKeysUntilRelease=True,bForceImmediately=False)"))

(fn ConstructionScript)